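; Enemy cannon actor that fires automatically when a Visibility trace between its two arrows hits the player pawn, checked every Tick.
; When loaded, it waits a random delay, spawns an EnemyCannonBall with explosion effect and random shot sound.
; Firetime and Reloadtime timelines offset the actor for firing and reloading, with the skeletal mesh walking during reload and idling once ready.
; The Reloading function only prints messages and sets a timer, uncalled here.
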(event Custom|Fire
  (bind _p_explosion_big_a (Variables|Default|GetP_Explosion_Big_A))
  (bind _skeletalmesh (Variables|Default|GetSkeletalMesh))
  (if (Variables|Default|Getisreload?)
    (Utilities|FlowControl|Delay (Math|Random|RandomFloatinRange 0.7 2.0))
    (Variables|Default|Setisreload? false)
    (Components|Activation|Activate _p_explosion_big_a false)
    (bind _returnvalue (Game|SpawnActorfromClass "/Game/My/asset/EnemyCannonBall.EnemyCannonBall_C" (Transformation|GetWorldTransform (Variables|Default|GetArrow)) "Undefined" "MultiplyWithRoot" 0 0))
    (Default|Fired _returnvalue)
    (Audio|PlaySoundatLocation (.OutItem (Utilities|Array|Random (Utilities|Array|MakeArray "/Game/My/asset/sound/배/cannon/AudioClip/cannon_big_single_2d_1.cannon_big_single_2d_1" "/Game/My/asset/sound/cannon-shot-14799.cannon-shot-14799" "/Game/My/asset/sound/배/cannon/AudioClip/cannon_big_single_2d_1.cannon_big_single_2d_1" "/Game/My/asset/sound/배/cannon/AudioClip/cannon_big_single_2d_2.cannon_big_single_2d_2" "/Game/My/asset/sound/배/cannon/AudioClip/cannon_big_single_2d_3.cannon_big_single_2d_3" "/Game/My/asset/sound/배/cannon/AudioClip/cannon_big_single_2d_4.cannon_big_single_2d_4" "/Game/My/asset/sound/배/cannon/AudioClip/cannon_big_single_2d_5.cannon_big_single_2d_5" "/Game/My/asset/sound/배/cannon/AudioClip/cannon_big_single_2d_6.cannon_big_single_2d_6" "/Game/My/asset/sound/배/cannon/AudioClip/cannon_big_single_3d_shot6.cannon_big_single_3d_shot6" "/Game/My/asset/sound/배/cannon/AudioClip/cannon_big_single_ver11_3d_shot4.cannon_big_single_ver11_3d_shot4" "/Game/My/asset/sound/배/cannon/AudioClip/cannon_big_single_2d_9c_3.cannon_big_single_2d_9c_3" "/Game/My/asset/sound/배/cannon/AudioClip/cannon_big_single_2d_9c_5.cannon_big_single_2d_9c_5" "/Game/My/asset/sound/배/cannon/AudioClip/cannon_big_single_ver11_3d_shot5.cannon_big_single_ver11_3d_shot5" "/Game/My/asset/sound/배/cannon/AudioClip/cannon_big_single_3d_shot2.cannon_big_single_3d_shot2" "/Game/My/asset/sound/배/cannon/AudioClip/cannon_big_single_3d_shot3.cannon_big_single_3d_shot3" "/Game/My/asset/sound/배/cannon/AudioClip/cannon_big_single_3d_shot1.cannon_big_single_3d_shot1"))) (Transformation|GetWorldLocation _p_explosion_big_a) "0, 0, 0" 1.0 1.0 0.0 0 0 0 0)
    (bind _새_트랙_0 (Timeline|firetime PlayFromStart)
      (:Update
        (Transformation|AddActorLocalOffset _새_트랙_0 false true))
      (:Finished
        (Components|Activation|Deactivate _p_explosion_big_a)
        (Utilities|FlowControl|Delay 5.0)
        (Utilities|FlowControl|Sequence
          (:then_0
            (bind _새_트랙_0_2 (Timeline|reloadtime PlayFromStart)
              (:Update
                (Transformation|AddActorLocalOffset _새_트랙_0_2 false true))
              (:Finished
                (Variables|Default|Setisreload? true)
                (Components|Animation|PlayAnimation _skeletalmesh "/Game/Pirate/Demoscene_UE4/Animations/ThirdPersonIdle.ThirdPersonIdle" true))))
          (:then_1
            (Components|Animation|PlayAnimation _skeletalmesh "/Game/Pirate/Demoscene_UE4/Animations/ThirdPersonWalk.ThirdPersonWalk" true)))))))

(event EventTick
  (params (DeltaSeconds :type Float%20%28single-precision%29))
  ;[1 1 1] 플래이어 감지 발사
  (bind _outhit (Collision|LineTraceByChannel (Transformation|GetWorldLocation (Variables|Default|GetArrow)) (Transformation|GetWorldLocation (Variables|Default|GetArrow1)) "TraceTypeQuery1" false 0 "None"))
  (if (== (.HitActor (Collision|BreakHitResult _outhit)) (Game|Player|GetPlayerPawn 0))
    (CallFunction|Fire)))

(fn ConstructionScript)

(fn Reloading
  (Development|PrintString "재장전중")
  (Utilities|Time|SetTimerbyEvent 0 1e+01)
  (Development|PrintString "재장전완료!"))