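; Cannon actor that fires CannonBall projectiles with explosion effects and randomized voice and shot sounds, gated by Isreload, which is true when loaded.
; Fire waits a short random delay, spawns the ball at the Arrow, then a timeline offsets the actor for recoil.
; After a pause, a second timeline moves it during reload while the skeletal mesh plays a walk animation, then restores readiness and idle.
; The separate Reloading function is an unused stub.
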(event Custom|Fire
  (bind _p_explosion_big_a (Variables|Default|GetP_Explosion_Big_A))
  (bind _skeletalmesh (Variables|Default|GetSkeletalMesh))
  (bind _returnvalue (Transformation|GetWorldLocation _p_explosion_big_a))
  (if (Variables|Default|Getisreload?)
    (Audio|PlaySoundatLocation (.OutItem (Utilities|Array|Random (Utilities|Array|MakeArray "/Game/My/asset/sound/사람/AudioClip/Fire_DS_1.Fire_DS_1" "/Game/My/asset/sound/사람/AudioClip/Fire_DS_2.Fire_DS_2" "/Game/My/asset/sound/사람/AudioClip/Fire_GR_1.Fire_GR_1" "/Game/My/asset/sound/사람/AudioClip/Fire_GR_2.Fire_GR_2" "/Game/My/asset/sound/사람/AudioClip/Fire_GR_3.Fire_GR_3" "/Game/My/asset/sound/사람/AudioClip/Fire_Z_4.Fire_Z_4"))) _returnvalue "0, 0, 0" 1.0 1.0 0.0 0 0 0 0)
    (Utilities|FlowControl|Delay (Math|Random|RandomFloatinRange 0.7 2.0))
    (Variables|Default|Setisreload? false)
    (Components|Activation|Activate _p_explosion_big_a false)
    (bind _returnvalue_2 (Game|SpawnActorfromClass "/Game/My/asset/CannonBall.CannonBall_C" (Transformation|GetWorldTransform (Variables|Default|GetArrow)) "Undefined" "MultiplyWithRoot" 0 0))
    (Default|Fired _returnvalue_2)
    (Audio|PlaySoundatLocation (.OutItem (Utilities|Array|Random (Utilities|Array|MakeArray "/Game/My/asset/sound/배/cannon/AudioClip/cannon_big_single_2d_1.cannon_big_single_2d_1" "/Game/My/asset/sound/cannon-shot-14799.cannon-shot-14799" "/Game/My/asset/sound/배/cannon/AudioClip/cannon_big_single_2d_1.cannon_big_single_2d_1" "/Game/My/asset/sound/배/cannon/AudioClip/cannon_big_single_2d_2.cannon_big_single_2d_2" "/Game/My/asset/sound/배/cannon/AudioClip/cannon_big_single_2d_3.cannon_big_single_2d_3" "/Game/My/asset/sound/배/cannon/AudioClip/cannon_big_single_2d_4.cannon_big_single_2d_4" "/Game/My/asset/sound/배/cannon/AudioClip/cannon_big_single_2d_5.cannon_big_single_2d_5" "/Game/My/asset/sound/배/cannon/AudioClip/cannon_big_single_2d_6.cannon_big_single_2d_6" "/Game/My/asset/sound/배/cannon/AudioClip/cannon_big_single_3d_shot6.cannon_big_single_3d_shot6" "/Game/My/asset/sound/배/cannon/AudioClip/cannon_big_single_ver11_3d_shot4.cannon_big_single_ver11_3d_shot4" "/Game/My/asset/sound/배/cannon/AudioClip/cannon_big_single_2d_9c_3.cannon_big_single_2d_9c_3" "/Game/My/asset/sound/배/cannon/AudioClip/cannon_big_single_2d_9c_5.cannon_big_single_2d_9c_5" "/Game/My/asset/sound/배/cannon/AudioClip/cannon_big_single_ver11_3d_shot5.cannon_big_single_ver11_3d_shot5" "/Game/My/asset/sound/배/cannon/AudioClip/cannon_big_single_3d_shot2.cannon_big_single_3d_shot2" "/Game/My/asset/sound/배/cannon/AudioClip/cannon_big_single_3d_shot3.cannon_big_single_3d_shot3" "/Game/My/asset/sound/배/cannon/AudioClip/cannon_big_single_3d_shot1.cannon_big_single_3d_shot1"))) _returnvalue "0, 0, 0" 1.0 1.0 0.0 0 0 0 0)
    (bind _새_트랙_0 (Timeline|firetime PlayFromStart)
      (:Update
        (Transformation|AddActorLocalOffset _새_트랙_0 false true))
      (:Finished
        (Development|PrintString "재장전 중!" true true "(R=0.000000,G=0.660000,B=1.000000,A=1.000000)" 9.0)
        (Components|Activation|Deactivate _p_explosion_big_a)
        (Utilities|FlowControl|Delay 5.0)
        (Utilities|FlowControl|Sequence
          (:then_0
            (bind _새_트랙_0_2 (Timeline|reloadtime PlayFromStart)
              (:Update
                (Transformation|AddActorLocalOffset _새_트랙_0_2 false true))
              (:Finished
                (Variables|Default|Setisreload? true)
                (Components|Animation|PlayAnimation _skeletalmesh "/Game/Pirate/Demoscene_UE4/Animations/ThirdPersonIdle.ThirdPersonIdle" true)
                (Development|PrintString "재장전 완료!")
                (Audio|PlaySoundatLocation (.OutItem (Utilities|Array|Random (Utilities|Array|MakeArray "/Game/My/asset/sound/사람/AudioClip/ready_GR_2.ready_GR_2" "/Game/My/asset/sound/사람/AudioClip/Deck_ready_sir_DS_1.Deck_ready_sir_DS_1" "/Game/My/asset/sound/사람/AudioClip/Cannons_prepared_GR_2.Cannons_prepared_GR_2" "/Game/My/asset/sound/사람/AudioClip/cannons_are_loaded_GR_1.cannons_are_loaded_GR_1" "/Game/My/asset/sound/사람/AudioClip/Prepared_DS_3.Prepared_DS_3"))) "0, 0, 0" "0, 0, 0" 1.0 1.0 0.0 0 0 0 0))))
          (:then_1
            (Components|Animation|PlayAnimation _skeletalmesh "/Game/Pirate/Demoscene_UE4/Animations/ThirdPersonWalk.ThirdPersonWalk" true)))))
    (else
      (Development|PrintString "아직 재장전 중입니다!"))))

(event EventTick
  (params (DeltaSeconds :type Float%20%28single-precision%29)))

(fn ConstructionScript)

(fn Reloading
  (Development|PrintString "재장전중")
  (Utilities|Time|SetTimerbyEvent 0 1e+01)
  (Development|PrintString "재장전완료!"))