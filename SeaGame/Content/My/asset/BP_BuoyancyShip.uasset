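; Player-controlled physics sailing ship with damage, sinking, repair and port/starboard cannon fire.
; Sail level and A/D keys drive force and torque each Tick, mouse buttons fire cannons tagged left or right, and FluidSim receives the hull's wake force.
; Cannonball overlaps drain health, then flooding raises a mass value that a timer applies to the mesh, leading to game over.
; E repairs and stops flooding; Q pumps out mass once flooding stops.
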(event Custom|질량관리
  ;[1 1 1] 질량 관리
  (Class|PrimitiveComponent|SetMassOverrideinKg (Variables|Default|GetStaticMesh) "None" (Variables|Default|Get배질량) true))

(event EventBeginPlay
  (bind _scene (Variables|Default|GetScene))
  ;[1 1 1] 파도
  (Audio|PlaySound2D "/Game/My/asset/sound/a-ship-sailing-in-the-red-sea-145666.a-ship-sailing-in-the-red-sea-145666" 0.6 1.0 0.0 0 0)
  (bind _fluidsim (Variables|Default|GetFluidSim)
    (:then
      (Default|RegisterDynamicForce _fluidsim (Utilities|Struct|MakeFluidForceDynamic "NewEnumerator0" 4.5e+02 1.0 _scene "/Water/FluidSimulation/Materials/Forces/M_Fluid_Sim_Force_Boat_Component.M_Fluid_Sim_Force_Boat_Component" (Utilities|Struct|MakeFluidForceSocketInfo (Utilities|Map|MakeMap "None" "None"))) _scene 0.0)
      ;[1 1 1] 질량 관리
      (Variables|Default|Set배질량 (Physics|GetMass (Variables|Default|GetStaticMesh)))
      (Utilities|Time|SetTimerbyEvent (delegate Custom|질량관리) 0.1 true))
    (:else)))

(event Collision|EventActorBeginOverlap
  (params (OtherActor :type Actor%20Object%20Reference))
  ;[1 1 1] 피격 판정
  (Audio|PlaySoundatLocation (.OutItem (Utilities|Array|Random (Utilities|Array|MakeArray "/Game/My/asset/sound/배/AudioClip/woodbroken/AudioClip/wood_destructive_random9.wood_destructive_random9" "/Game/My/asset/sound/배/AudioClip/cannonball_impact_wood_hard_15.cannonball_impact_wood_hard_15" "/Game/My/asset/sound/배/AudioClip/woodbroken/AudioClip/wood_destructive_random7.wood_destructive_random7" "/Game/My/asset/sound/배/AudioClip/woodbroken/AudioClip/wood_destructive_random10.wood_destructive_random10"))) (Transformation|GetActorLocation OtherActor) "0, 0, 0" 1.0 1.0 0.0 0 0 0 0)
  (Utilities|Casting|CastToEnemyCannonBall OtherActor)
  (if (>= (- (Variables|Default|Get체력) 1) 0)
    (Variables|Default|Set체력 (- (Variables|Default|Get체력) 1))
    (else
      (Variables|Default|Setsinking true)
      ;[1 1 1] 침몰
      (Utilities|FlowControl|Delay 1.0 :!label _label)
      (if (Variables|Default|Getsinking)
        (bind _output_get (Variables|Default|Set배질량 (+ (Variables|Default|Get배질량) 3e+02)))
        (Development|PrintString "꼬르륵")
        ;[1 1 1] 게임오버 시퀸스
        (if (>= _output_get 4.2e+03)
          (Actor|DestroyActor (Actor|GetAttachedActors true true))
          (bind _foundwidgets (Widget|GetAllWidgetsOfClass "/Game/My/asset/hud/TextStoryWidget.TextStoryWidget_C" true))
          (Widget|RemovefromParent _foundwidgets)
          (Utilities|FlowControl|Delay 4.0)
          (bind _returnvalue (UserInterface|CreateWidget "/Game/My/asset/hud/GameOverWidget.GameOverWidget_C"))
          (UserInterface|Viewport|AddtoViewport _returnvalue 0)
          (else
            (goto _label)))))))

(event EventTick
  (params (DeltaSeconds :type Float%20%28single-precision%29))
  ;[1 1 1] 기동 로직
  (Physics|AddForce (Variables|Default|GetStaticMesh) (* (* (Variables|Default|Getsailgrade) (Transformation|GetActorForwardVector)) "100.000000,100.000000,0.000000") "None" true)
  (if (Variables|Default|Geta%20)
    (Class|PrimitiveComponent|AddTorqueinDegrees (Variables|Default|GetStaticMesh) (* (Transformation|GetActorUpVector) -10) "None" true))
  (if (Variables|Default|Getd)
    (Class|PrimitiveComponent|AddTorqueinDegrees (Variables|Default|GetStaticMesh) (* (Transformation|GetActorUpVector) 10) "None" true)))

(event Input|MouseEvents|MouseX
  (params (AxisValue :type Float%20%28single-precision%29))
  ;[1 1 1] 카메라 움직임
  (Pawn|Input|AddControllerYawInput AxisValue))

(event Input|MouseEvents|MouseY
  (params (AxisValue :type Float%20%28single-precision%29))
  ;[1 1 1] 카메라 움직임
  (Pawn|Input|AddControllerPitchInput AxisValue))

(event Input|KeyboardEvents|W
  (params (Key :type Key%20Structure :default "None"))
  ;[1 1 1] 전진 정지
  (:Released
    (bind _output_get (Variables|Default|Setsailgrade (Math|Integer|Clamp(Integer) (+ (Variables|Default|Getsailgrade) 1) 0 3)))
    (Development|PrintString (Utilities|String|Append "돛 :" (Utilities|String|ToString(Integer) _output_get)))))

(event Input|MouseEvents|LeftMouseButton
  (params (Key :type Key%20Structure :default "None"))
  ;[1 1 1] 대포 사격
  (:Pressed
    (Development|PrintString "left")
    (bind _outactors (Actor|GetAllActorsOfClasswithTag "/Game/My/asset/cannon/BP_Cannon.BP_Cannon_C" "left"))
    (Default|Fire _outactors)))

(event Input|KeyboardEvents|S
  (params (Key :type Key%20Structure :default "None"))
  ;[1 1 1] 전진 정지
  (:Released
    (bind _output_get (Variables|Default|Setsailgrade (Math|Integer|Clamp(Integer) (- (Variables|Default|Getsailgrade) 1) 0 3)))
    (Development|PrintString (Utilities|String|Append "돛 :" (Utilities|String|ToString(Integer) _output_get)))))

(event Input|KeyboardEvents|A
  (params (Key :type Key%20Structure :default "None"))
  ;[1 1 1] 좌우 버튼반응
  (:Pressed
    (Variables|Default|Seta%20 true))
  (:Released
    (Variables|Default|Seta%20 false)))

(event Input|KeyboardEvents|D
  (params (Key :type Key%20Structure :default "None"))
  ;[1 1 1] 좌우 버튼반응
  (:Pressed
    (Variables|Default|Setd true))
  (:Released
    (Variables|Default|Setd false)))

(event Input|MouseEvents|RightMouseButton
  (params (Key :type Key%20Structure :default "None"))
  ;[1 1 1] 대포 사격
  (:Pressed
    (Development|PrintString "right")
    (bind _outactors (Actor|GetAllActorsOfClasswithTag "/Game/My/asset/cannon/BP_Cannon.BP_Cannon_C" "right"))
    (Default|Fire _outactors)))

(event Input|KeyboardEvents|Q
  (params (Key :type Key%20Structure :default "None"))
  ;[1 1 1] 배수 펌프 작동
  (:Pressed
    (if (stale _output_get)
      (Development|PrintString "펌프가 바쁩니다..")
      (else
        (if (Variables|Default|Getsinking) :!label _label
          (Development|PrintString "배에 물이들어오고 있습니다. 수리를 먼저 해주세요.")
          (Variables|Default|Set펌프%20작동 false)
          (else
            (Development|PrintString "펌프 작동.")
            (bind _output_get (Variables|Default|Set펌프%20작동 true))
            (if (<= (- (Variables|Default|Get배질량) 3e+01) 5e+01)
              (Development|PrintString "더이상 물을 뺼수 없습니다!")
              (Variables|Default|Set펌프%20작동 false)
              (else
                (Development|PrintString (Utilities|String|ToString(Float) (- (Variables|Default|Get배질량) 3e+01)))
                (Variables|Default|Set배질량 (- (Variables|Default|Get배질량) 3e+01))
                (Utilities|FlowControl|Delay 0.4)
                (goto _label)))))))))

(event Input|KeyboardEvents|E
  (params (Key :type Key%20Structure :default "None"))
  ;[1 1 1] 수리
  (:Pressed
    (Audio|PlaySound2D "/Game/My/asset/sound/wood-door-knock-106669.wood-door-knock-106669" 2.0 1.0 0.0 0 0)
    (if (<= (+ (Variables|Default|Get체력) 1) 10)
      (Development|PrintString "수리중입니다..")
      (bind _output_get (Variables|Default|Set체력 (+ (Variables|Default|Get체력) 1)))
      (Variables|Default|Setsinking false)
      (Development|PrintString (Utilities|String|Append "체력:" (Utilities|String|ToString(Integer) _output_get)))
      (else
        (Development|PrintString "이미 수리가 끝났습니다.")))))

(fn ConstructionScript)

(fn 퀘스트진행)