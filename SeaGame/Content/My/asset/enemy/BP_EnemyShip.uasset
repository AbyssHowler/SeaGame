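; Enemy ship pawn that chases the player, takes CannonBall hits and sinks when health runs out.
; Tick pushes the physics mesh forward, snapping rotation toward distant players and, up close, torquing it by the sensed pawn's world-axis quadrant.
; PawnSensing, enabled after a BeginPlay delay, supplies that pawn.
; Sinking uses a looping timer to add mass until a threshold, then destroys the ship and updates kill and spawn manager counts.
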(event OnSeePawn(PawnSensing)
  (params (Pawn :type Pawn%20Object%20Reference))
  ;[1 1 1] 적 AI추적 매커니즘
  ;;[1 1 1] 플레이어 감지
  (Variables|Default|Setissee? true)
  (Variables|Default|Setright false))

(event Custom|sinking!
  (bind _staticmesh (Variables|Default|GetStaticMesh))
  (bind _returnvalue (Physics|GetMass _staticmesh))
  ;[1 1 1] 침몰
  (if (Variables|Default|Getsinking)
    (Class|PrimitiveComponent|SetMassOverrideinKg _staticmesh "None" (+ _returnvalue 3.0) true)
    (if (>= _returnvalue 9e+02)
      (Actor|DestroyActor (Actor|GetAttachedActors true true))
      (Utilities|FlowControl|Delay 4.0)
      (bind _returnvalue_2 (Actor|GetActorOfClass "/Game/My/asset/BP_KIllCountManager.BP_KIllCountManager_C"))
      (Variables|/Game/My/asset/BP_KIllCountManager.BP_KIllCountManager_C|SetKillCount _returnvalue_2 (+ (Variables|/Game/My/asset/BP_KIllCountManager.BP_KIllCountManager_C|GetKillCount _returnvalue_2) 1))
      (Variables|/Game/My/asset/BP_SpawnManager.BP_SpawnManager_C|SetenemyCount (stale EventBeginPlay _asbp_spawn_manager) (+ (Variables|/Game/My/asset/BP_SpawnManager.BP_SpawnManager_C|GetenemyCount (stale EventBeginPlay _asbp_spawn_manager)) -1))
      (Actor|DestroyActor))))

(event Collision|EventActorBeginOverlap
  (params (OtherActor :type Actor%20Object%20Reference))
  ;[1 1 1] 피격
  (Utilities|Casting|CastToCannonBall OtherActor)
  (if (>= (- (Variables|Default|Get체력) 1) 0)
    (bind _output_get (Variables|Default|Set체력 (- (Variables|Default|Get체력) 1)))
    (Development|PrintString (Utilities|String|Append "적체력: " (Utilities|String|ToString(Integer) _output_get)))
    (else
      (Development|PrintString "적 격침!")
      (Variables|Default|Setsinking true)
      (Utilities|Time|SetTimerbyEvent (delegate Custom|sinking!) 0.1 true))))

(event EventTick
  (params (DeltaSeconds :type Float%20%28single-precision%29))
  (bind _returnvalue (Game|Player|GetPlayerPawn 0))
  (bind _returnvalue_2 (Transformation|GetActorLocation))
  (bind _returnvalue_3 (Transformation|GetActorLocation _returnvalue))
  (bind _returnvalue_4 (Math|Rotator|FindLookatRotation _returnvalue_3 _returnvalue_2))
  (bind (_roll _pitch _yaw) (Math|Rotator|BreakRotator _returnvalue_4))
  ;[1 1 1] 적 AI추적 매커니즘
  ;;[1 1 1] 장거리 적 추적
  (Physics|AddForce (Variables|Default|GetStaticMesh) (* (* "3.000000,3.000000,3.000000" (Transformation|GetActorForwardVector)) "100.000000,100.000000,0.000000") "None" true)
  (if (>= (Transformation|GetDistanceTo _returnvalue) (Variables|Default|Get접근거리))
    (Transformation|SetActorRotation (Math|Rotator|MakeRotator _roll _pitch (+ _yaw 1.8e+02)))
    (elif (> 0.0 (- (.X (Math|Vector|BreakVector (Transformation|GetActorLocation (stale OnSeePawn(PawnSensing) Pawn)))) (.X (Math|Vector|BreakVector (Transformation|GetWorldLocation (Variables|Default|GetStaticMesh))))))
      ;;[1 1 1] 1,2사분면-> 꺽어서 공격
      (if (> (- (.Y (Math|Vector|BreakVector (Transformation|GetActorLocation (stale OnSeePawn(PawnSensing) Pawn)))) (.Y (Math|Vector|BreakVector (Transformation|GetWorldLocation (Variables|Default|GetStaticMesh))))) 0.0) ; 12
        (Class|PrimitiveComponent|AddTorqueinDegrees (Variables|Default|GetStaticMesh) (* (Transformation|GetActorUpVector) 10) "None" true)
        (else
          (Class|PrimitiveComponent|AddTorqueinDegrees (Variables|Default|GetStaticMesh) (* (Transformation|GetActorUpVector) -10) "None" true)))
      (else
        ;;[1 1 1] 3,4사분면 ->플레이어 포워드 좌표 동일하게
        (if (> (- (.Y (Math|Vector|BreakVector (Transformation|GetActorLocation (stale OnSeePawn(PawnSensing) Pawn)))) (.Y (Math|Vector|BreakVector (Transformation|GetWorldLocation (Variables|Default|GetStaticMesh))))) 0.0) ; 34
          (if (> (- (.Y (Math|Vector|BreakVector (Transformation|GetActorForwardVector (stale OnSeePawn(PawnSensing) Pawn)))) (.Y (Math|Vector|BreakVector (Transformation|GetActorForwardVector)))) 0.0) ; 3
            (Class|PrimitiveComponent|AddTorqueinDegrees (Variables|Default|GetStaticMesh) (* (Transformation|GetActorUpVector) 10) "None" true)
            (else
              (Class|PrimitiveComponent|AddTorqueinDegrees (Variables|Default|GetStaticMesh) (* (Transformation|GetActorUpVector) -10) "None" true)))
          (elif (> (- (.Y (Math|Vector|BreakVector (Transformation|GetActorForwardVector (stale OnSeePawn(PawnSensing) Pawn)))) (.Y (Math|Vector|BreakVector (Transformation|GetActorForwardVector)))) 0.0) ; 4
            (Class|PrimitiveComponent|AddTorqueinDegrees (Variables|Default|GetStaticMesh) (* (Transformation|GetActorUpVector) 10) "None" true)
            (else
              (Class|PrimitiveComponent|AddTorqueinDegrees (Variables|Default|GetStaticMesh) (* (Transformation|GetActorUpVector) -10) "None" true))))))))

(event EventBeginPlay
  ;[1 1 1] 스폰관리
  (bind _returnvalue (Actor|GetActorOfClass "/Game/My/asset/BP_SpawnManager.BP_SpawnManager_C"))
  (bind _asbp_spawn_manager (Utilities|Casting|CastToBP_SpawnManager _returnvalue))
  (Variables|/Game/My/asset/BP_SpawnManager.BP_SpawnManager_C|SetenemyCount _asbp_spawn_manager (+ (Variables|/Game/My/asset/BP_SpawnManager.BP_SpawnManager_C|GetenemyCount _asbp_spawn_manager) 1))
  (bind _asai_컨트롤러 (Utilities|Casting|CastToAIController (Pawn|GetController)))
  (Development|PrintString (Utilities|GetDisplayName _asai_컨트롤러))
  (Utilities|FlowControl|Delay 3.0)
  (Class|PawnSensingComponent|SetSensingUpdatesEnabled (Variables|Default|GetPawnSensing) true))

(fn ConstructionScript)